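; BP_PuzzleQuestHUD creates the Puzzle Quest HUD widget and displays the player's knight stats on screen.
; On BeginPlay it adds W_PuzzleQuestHUD to the viewport, reads initial stats from player 0's PuzzleQuestPlayerState and binds to its OnStatsChanged event.
; Initial values and later changes go through UpdateHUDValues, which writes stamina and max health, rather than current health, into the stamina and health text fields.
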(event Custom|OnStatsChanged
  (params (PlayerStats :type Player%20Stats%20Structure))
  (CallFunction|UpdateHUDValues PlayerStats))

(event EventBeginPlay
  (bind _returnvalue (UserInterface|CreateWidget "/Game/W_PuzzleQuestHUD.W_PuzzleQuestHUD_C"))
  (bind _output_get (Variables|Default|SetPuzzleQuestWidget _returnvalue))
  (UserInterface|Viewport|AddtoViewport _output_get 0)
  (bind _aspuzzle_quest_player_state (Utilities|Casting|CastToPuzzleQuestPlayerState (Game|GetPlayerState 0)))
  (bind _returnvalue_2 (Class|PuzzleQuestPlayerState|GetPlayerStats _aspuzzle_quest_player_state))
  (CallFunction|UpdateHUDValues _returnvalue_2)
  (EventDispatchers|BindEventtoOnStatsChanged _aspuzzle_quest_player_state (delegate Custom|OnStatsChanged)))

(fn ConstructionScript)

(fn UpdateHUDValues
  (params (PlayerStats :type Player%20Stats%20Structure))
  (bind _puzzlequestwidget (Variables|Default|GetPuzzleQuestWidget))
  (Variables|/Script/UMG.TextBlock|SetText (Variables|/Game/W_PuzzleQuestHUD.W_PuzzleQuestHUD_C|GetStaminaValue _puzzlequestwidget) (Utilities|Text|ToText(String) (.knightstamina PlayerStats)))
  (Variables|/Script/UMG.TextBlock|SetText (Variables|/Game/W_PuzzleQuestHUD.W_PuzzleQuestHUD_C|GetHealthValue _puzzlequestwidget) (Utilities|Text|ToText(String) (.knightmaxhealth PlayerStats))))